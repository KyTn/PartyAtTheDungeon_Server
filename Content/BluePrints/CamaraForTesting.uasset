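; Test camera Blueprint for checking whether a referenced ActorToTest projects onto the player's screen.
; CalculateFrustum projects that actor's location through player controller 0, prints the success flag and screen position, and returns the flag.
; Despite the name, it does no frustum or screen-bounds math, and the CameraComponent view it fetches goes unused.
; The event graph and construction script are empty, so nothing here calls the function.
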(event EventBeginPlay)

(event Collision|EventActorBeginOverlap
  (params (OtherActor :type Actor%20Object%20Reference)))

(event EventTick
  (params (DeltaSeconds :type Float%20%28single-precision%29)))

(fn ConstructionScript)

(fn CalculateFrustum
  (bind _returnvalue (Game|GetPlayerController 0))
  (bind _actortotest (Variables|Default|GetActorToTest))
  (bind _returnvalue_2 (Transformation|GetActorLocation _actortotest))
  (bind (_screenposition _returnvalue_3) (Class|GameplayStatics|ProjectWorldtoScreen _returnvalue _returnvalue_2 false))
  (bind _desiredview (Class|CameraComponent|GetCameraView (Variables|CameraActor|GetCameraComponent) 0.0))
  (Development|PrintString (Utilities|String|ToString(Boolean) _returnvalue_3))
  (Development|PrintString (Utilities|String|ToString(Vector2d) _screenposition))
  (return _returnvalue_3))