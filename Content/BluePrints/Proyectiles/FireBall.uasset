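; Fireball projectile that moves forward along its facing each tick at a set velocity without sweeping, playing a launch sound on spawn.
; Overlapping a PD_E_Character other than its instigator applies damage, destroys the fireball and plays an explosion.
; A kill also credits the instigator character with the victim's points and a defeated enemy.
; Overlapping a PD_E_WallActor destroys it silently; debug prints remain in the overlap logic.
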(event EventBeginPlay
  (Audio|PlaySound2D "/Game/Music/FX_Skills/fireball_launch.fireball_launch"))

(event Collision|EventActorBeginOverlap
  (params (OtherActor :type Actor%20Object%20Reference))
  (bind _returnvalue (Game|GetInstigator))
  (Development|PrintString (Utilities|GetObjectName OtherActor) true true "(R=1.000000,G=0.821623,B=0.000000,A=1.000000)")
  (bind _aspd_e_character (Utilities|Casting|CastToPD_E_Character OtherActor)
    (:then
      (if (!= _aspd_e_character _returnvalue)
        (bind _result (Math|Float|NegateFloat (Variables|Default|GetDamage))
          (:%20%20
            (Class|PDECharacter|UpdateCharLife _aspd_e_character _result)
            (bind _returnvalue_2 (Class|PDECharacter|IsDead _aspd_e_character))
            (if _returnvalue_2
              (Development|PrintString "Hello fireball")
              (bind _returnvalue_3 (Class|PDECharacter|GetPoints _aspd_e_character))
              (bind _aspd_e_character_2 (Utilities|Casting|CastToPD_E_Character _returnvalue))
              (Class|PDECharacter|UpdatePoints _aspd_e_character_2 _returnvalue_3)
              (Class|PDECharacter|UpdateEnemiesDefeated _aspd_e_character_2))
            (Actor|DestroyActor)
            (Audio|PlaySoundatLocation "/Game/Music/FX_Skills/explosion.explosion" (Transformation|GetActorLocation))))))
    (:CastFailed
      (Utilities|Casting|CastToPD_E_WallActor OtherActor)
      (Actor|DestroyActor))))

(event EventTick
  (params (DeltaSeconds :type Float%20%28single-precision%29))
  (Transformation|SetActorLocation (+ (Transformation|GetActorLocation) (* (Transformation|GetActorForwardVector) (* DeltaSeconds (Variables|Default|GetVelocity)))) false false))

(fn ConstructionScript)