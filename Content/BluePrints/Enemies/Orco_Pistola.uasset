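; Gunslinger orc enemy character that wields two guns, spawned at BeginPlay on its hand sockets and set to simulate physics on destruction.
; Capsule overlaps with other characters trigger collision handling, and Tick plays a skill animation while collision-stopped, otherwise deactivating the skill particle.
; Skill types select particle effects, the widget receives a character reference, and a function blends the player's view to this orc.
; Wall-avoidance rotation and critical-attack animation logic are disconnected.
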(event OnComponentBeginOverlap(Capsule)
  (params (OverlappedComponent :type Primitive%20Component%20Object%20Reference) (OtherActor :type Actor%20Object%20Reference) (OtherComp :type Primitive%20Component%20Object%20Reference) (OtherBodyIndex :type Integer) (bFromSweep :type Boolean) (SweepResult :type Hit%20Result%20Structure%20%28by%20ref%29))
  (bind _aspd_e_character (Utilities|Casting|CastToPD_E_Character OtherActor))
  (Development|PrintText "PistoleroOverlapeando")
  (Class|PDECharacter|CollisionwithOtherCharacter _aspd_e_character))

(event EventBeginPlay
  (bind _returnvalue (Math|Transform|MakeTransform "0, 0, 0" "0, 0, 0" "1.000000,1.000000,1.000000"))
  (bind _mesh (Variables|Character|GetMesh))
  (Utilities|FlowControl|Sequence
    (:then_0
      ;[0 0 1] 2 Pistolas
      (bind _returnvalue_2 (Game|SpawnActorfromClass "/Game/BluePrints/Weapons/GunWeapon.GunWeapon_C" _returnvalue "Undefined" 0 0))
      (Variables|Default|SetWeapon_ _returnvalue_2)
      (bind _returnvalue_3 (Game|SpawnActorfromClass "/Game/BluePrints/Weapons/GunWeapon.GunWeapon_C" _returnvalue "Undefined" 0 0))
      (Variables|Default|SetWeapon_1 _returnvalue_3)
      (Transformation|AttachComponentToComponent (Variables|/Game/BluePrints/Weapons/GunWeapon.GunWeapon_C|GetWeapon _returnvalue_2) _mesh "RightHand" "KeepRelative" "KeepRelative" "KeepRelative" true)
      (Transformation|AttachComponentToComponent (Variables|/Game/BluePrints/Weapons/GunWeapon.GunWeapon_C|GetWeapon _returnvalue_3) _mesh "LeftHand" "KeepRelative" "KeepRelative" "KeepRelative" true))
    (:then_1
      (bind _asui_s_widget_character (Utilities|Casting|CastToUI_S_WidgetCharacter (UserInterface|GetUserWidgetObject (Variables|Default|GetWidget))))
      (Variables|/Game/UserInterface/UI_Server/UI_S_WidgetCharacter.UI_S_WidgetCharacter_C|SetCharacterRef _asui_s_widget_character self))))

(event Collision|EventActorBeginOverlap
  (params (OtherActor :type Actor%20Object%20Reference)))

(event EventTick
  (params (DeltaSeconds :type Float%20%28single-precision%29))
  ;[1 1 1] Rotar la camara del character para que nunca pille muro
  (Utilities|FlowControl|Sequence
    (:then_0
      (bind _returnvalue (Class|PDECharacter|IscharacterStoppingbyCollision))
      (if _returnvalue
        (Class|PDECharacter|PlayAnimationSkill 249)
        (else
          (Components|Activation|Deactivate (Variables|Default|GetParticleSKill)))))))

(event EventDestroyed
  ;[1 1 1] Dejar caer el arma cuando muere
  (bind _asgun_weapon (Utilities|Casting|CastToGunWeapon (Variables|Default|GetWeapon_)))
  (Physics|SetSimulatePhysics (Variables|/Game/BluePrints/Weapons/GunWeapon.GunWeapon_C|GetWeapon _asgun_weapon) true)
  (bind _asgun_weapon_2 (Utilities|Casting|CastToGunWeapon (Variables|Default|GetWeapon_1)))
  (Physics|SetSimulatePhysics (Variables|/Game/BluePrints/Weapons/GunWeapon.GunWeapon_C|GetWeapon _asgun_weapon_2) true))

(fn ConstructionScript)

(fn PlaySkillAnimation
  (params (Skill :type Integer))
  (bind _particleskill (Variables|Default|GetParticleSKill))
  (bind _particleskill_2 (Variables|Default|GetParticleSKill))
  (bind _particleskill_3 (Variables|Default|GetParticleSKill))
  (bind _particleskill_4 (Variables|Default|GetParticleSKill))
  (switch Utilities|FlowControl|Switch|SwitchonActiveSkills (Utilities|Enum|ByteToEnumActiveSkills (Math|Conversions|ToByte(Integer) Skill))
    (:BasicAttack
      ;[1 1 1] Ataque básico
      (Effects|Components|ParticleSystem|SetTemplate _particleskill "/Game/InfinityBladeEffects/Effects/FX_Combat_Base/WeaponCombo/P_Combo_Finish_Untyped_01.P_Combo_Finish_Untyped_01")
      (Components|Activation|Activate _particleskill false))
    (:Defense
      ;[1 1 1] Defense
      (Effects|Components|ParticleSystem|SetTemplate _particleskill "/Game/InfinityBladeEffects/Effects/FX_Ability/Heal/P_Health_Pickup_01.P_Health_Pickup_01")
      (Components|Activation|Activate _particleskill false))
    (:WhenFua
      ;[1 1 1] WhenFUA
      (Effects|Components|ParticleSystem|SetTemplate _particleskill "/Game/InfinityBladeEffects/Effects/FX_Skill_Aura/WhenFua.WhenFua")
      (Components|Activation|Activate _particleskill false))
    (:WhoHeal
      ;[1 1 1] Heal and ShotMana
      (Effects|Components|ParticleSystem|SetTemplate _particleskill_4 "/Game/InfinityBladeEffects/Effects/FX_Ability/Heal/P_Heal_Target.P_Heal_Target" :!label _label)
      (Components|Activation|Activate _particleskill_4 false))
    (:ShotMana
      (goto _label))
    (:GetStunnedByCollision
      ;[1 1 1] Get Stunned by Collision
      (Effects|Components|ParticleSystem|SetTemplate _particleskill_3 "/Game/InfinityBladeEffects/Effects/FX_Ability/Stun/P_Stun_Collision.P_Stun_Collision")
      (Components|Activation|Activate _particleskill_3 false))
    (:GetHurt
      ;[1 1 1] Get Hurt
      (Effects|Components|ParticleSystem|SetTemplate _particleskill_2 "/Game/InfinityBladeEffects/Effects/FX_Ability/Stun/P_Stun_Stars_Base.P_Stun_Stars_Base")
      (Components|Activation|Activate _particleskill_2 false))))

(fn PutCameraPlayeronView
  (Variables|Default|SetbFindCameraComponentWhenViewTarget true)
  (Game|Player|SetViewTargetwithBlend (Game|GetPlayerController 0) self 0.5 "VTBlend_EaseInOut" 0.0 false))

(fn StopParticleSystem
  (Components|Activation|Deactivate (Variables|Default|GetParticleSKill)))