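; Orc archer enemy character that spawns a bow in its left hand, links its overhead widget and drops the bow with physics when destroyed.
; PlaySkillAnimation maps each skill to a particle effect, while Tick polls collision-stop state to trigger a skill animation or deactivate the particles.
; Capsule overlaps with other characters call the collision handler, and a helper blends the player's view to this character.
; Wall-camera rotation, widget naming and critical-attack animation chains are unwired.
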(event OnComponentBeginOverlap(Capsule)
  (params (OverlappedComponent :type Primitive%20Component%20Object%20Reference) (OtherActor :type Actor%20Object%20Reference) (OtherComp :type Primitive%20Component%20Object%20Reference) (OtherBodyIndex :type Integer) (bFromSweep :type Boolean) (SweepResult :type Hit%20Result%20Structure%20%28by%20ref%29))
  (bind _aspd_e_character (Utilities|Casting|CastToPD_E_Character OtherActor))
  (Development|PrintText "Arquero overlapeando")
  (Class|PDECharacter|CollisionwithOtherCharacter _aspd_e_character))

(event EventBeginPlay
  (Utilities|FlowControl|Sequence
    (:then_0
      ;[0 0 1] ARCO
      (bind _returnvalue (Game|SpawnActorfromClass "/Game/BluePrints/Weapons/BowWeapon.BowWeapon_C" (Math|Transform|MakeTransform "0, 0, 0" "0, 0, 0" "2.000000,2.000000,2.000000") "Undefined" 0 0))
      (Variables|Default|SetWeapon_ _returnvalue)
      (Transformation|AttachComponentToComponent (Variables|/Game/BluePrints/Weapons/BowWeapon.BowWeapon_C|GetWeapon _returnvalue) (Variables|Character|GetMesh) "LeftHand" "KeepRelative" "KeepRelative" "KeepRelative" true))
    (:then_1
      (bind _asui_s_widget_character (Utilities|Casting|CastToUI_S_WidgetCharacter (UserInterface|GetUserWidgetObject (Variables|Default|GetWidget))))
      (Variables|/Game/UserInterface/UI_Server/UI_S_WidgetCharacter.UI_S_WidgetCharacter_C|SetCharacterRef _asui_s_widget_character self))))

(event Collision|EventActorBeginOverlap
  (params (OtherActor :type Actor%20Object%20Reference)))

(event EventTick
  (params (DeltaSeconds :type Float%20%28single-precision%29))
  ;[1 1 1] Rotar la camara del character para que nunca pille muro
  (Utilities|FlowControl|Sequence
    (:then_0
      (bind _returnvalue (Class|PDECharacter|IscharacterStoppingbyCollision))
      (if _returnvalue
        (Class|PDECharacter|PlayAnimationSkill 249)
        (else
          (Components|Activation|Deactivate (Variables|Default|GetParticleSKill)))))))

(event EventDestroyed
  ;[1 1 1] Dejar caer el arma cuando muere
  (bind _asbow_weapon (Utilities|Casting|CastToBowWeapon (Variables|Default|GetWeapon_)))
  (Physics|SetSimulatePhysics (Variables|/Game/BluePrints/Weapons/BowWeapon.BowWeapon_C|GetWeapon _asbow_weapon) true))

(fn ConstructionScript)

(fn PlaySkillAnimation
  (params (skill :type Integer))
  (bind _particleskill (Variables|Default|GetParticleSKill))
  (bind _particleskill_2 (Variables|Default|GetParticleSKill))
  (bind _particleskill_3 (Variables|Default|GetParticleSKill))
  (bind _particleskill_4 (Variables|Default|GetParticleSKill))
  (bind _particleskill_5 (Variables|Default|GetParticleSKill))
  (switch Utilities|FlowControl|Switch|SwitchonActiveSkills (Utilities|Enum|ByteToEnumActiveSkills (Math|Conversions|ToByte(Integer) skill))
    (:BasicAttack
      ;[1 1 1] Ataque básico
      (Effects|Components|ParticleSystem|SetTemplate _particleskill "/Game/InfinityBladeEffects/Effects/FX_Combat_Base/WeaponCombo/P_Combo_Finish_Untyped_01.P_Combo_Finish_Untyped_01" :!label _label)
      (Components|Activation|Activate _particleskill false))
    (:Defense
      ;[1 1 1] Defense
      (Effects|Components|ParticleSystem|SetTemplate _particleskill "/Game/InfinityBladeEffects/Effects/FX_Ability/Heal/P_Health_Pickup_01.P_Health_Pickup_01")
      (Components|Activation|Activate _particleskill false))
    (:WhenFua
      ;[1 1 1] WhenFUA
      (Effects|Components|ParticleSystem|SetTemplate _particleskill_4 "/Game/InfinityBladeEffects/Effects/FX_Skill_Aura/WhenFua.WhenFua")
      (Components|Activation|Activate _particleskill_4 false))
    (:Hostion
      (goto _label))
    (:WhoHeal
      ;[1 1 1] Heal and ShotMana
      (Effects|Components|ParticleSystem|SetTemplate _particleskill_5 "/Game/InfinityBladeEffects/Effects/FX_Ability/Heal/P_Heal_Target.P_Heal_Target" :!label _label_2)
      (Components|Activation|Activate _particleskill_5 false))
    (:ShotMana
      (goto _label_2))
    (:GetStunnedByCollision
      ;[1 1 1] Get Stunned by Collision
      (Effects|Components|ParticleSystem|SetTemplate _particleskill_2 "/Game/InfinityBladeEffects/Effects/FX_Ability/Stun/P_Stun_Collision.P_Stun_Collision")
      (Components|Activation|Activate _particleskill_2 false))
    (:GetHurt
      ;[1 1 1] Get Hurt
      (Effects|Components|ParticleSystem|SetTemplate _particleskill_3 "/Game/InfinityBladeEffects/Effects/FX_Ability/Stun/P_Stun_Stars_Base.P_Stun_Stars_Base")
      (Components|Activation|Activate _particleskill_3 false))))

(fn PutCameraPlayeronView
  (Variables|Default|SetbFindCameraComponentWhenViewTarget true)
  (Game|Player|SetViewTargetwithBlend (Game|GetPlayerController 0) self 0.5 "VTBlend_EaseInOut" 0.0 false))

(fn StopParticleSystem
  (Components|Activation|Deactivate (Variables|Default|GetParticleSKill)))