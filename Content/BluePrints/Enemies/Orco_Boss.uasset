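; Orc boss enemy Blueprint that handles skill visuals and its own camera view.
; PlaySkillAnimation maps each skill to a particle template on a shared component, except Fire Blast, which spawns a FireBall actor.
; PutCameraPlayerOnView blends the player's view to the boss, while Tick traces camera-to-mesh and swings the spring arm 180 degrees in yaw when a wall actor blocks it.
; Weapon-drop physics and critical-attack animation nodes are unconnected.
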(event EventBeginPlay)

(event Collision|EventActorBeginOverlap
  (params (OtherActor :type Actor%20Object%20Reference)))

(event EventDestroyed
  ;[1 1 1] Dejar caer las armas cuando muera el character+
)

(event EventTick
  (params (DeltaSeconds :type Float%20%28single-precision%29))
  (bind _springarm (Variables|Default|GetSpringArm))
  (bind _returnvalue (Transformation|GetWorldRotation _springarm))
  (bind (_roll _pitch _yaw) (Math|Rotator|BreakRotator _returnvalue))
  ;[1 1 1] Rotar la camara del character para que nunca pille muro
  (bind _outhit (Collision|LineTraceForObjects (Transformation|GetWorldLocation (Variables|Default|GetCamera)) (Transformation|GetWorldLocation (Variables|Character|GetMesh)) (Utilities|Array|MakeArray "ObjectTypeQuery1") false 0 "None" false))
  (Utilities|Casting|CastToBP_ME_WallActor (.HitActor (Collision|BreakHitResult _outhit)))
  (Transformation|SetRelativeRotation _springarm (Math|Rotator|MakeRotator _roll _pitch (+ _yaw 1.8e+02)) true false))

(fn ConstructionScript)

(fn PlaySkillAnimation
  (params (Skill :type Integer))
  (bind _particleskill (Variables|Default|GetParticleSKill))
  (bind _particleskill_2 (Variables|Default|GetParticleSKill))
  (bind _particleskill_3 (Variables|Default|GetParticleSKill))
  (bind _particleskill_4 (Variables|Default|GetParticleSKill))
  (switch Utilities|FlowControl|Switch|SwitchonActiveSkills (Utilities|Enum|ByteToEnumActiveSkills (Math|Conversions|ToByte(Integer) Skill))
    (:BasicAttack
      ;[1 1 1] Ataque básico
      (Effects|Components|ParticleSystem|SetTemplate _particleskill "/Game/InfinityBladeEffects/Effects/FX_Combat_Base/WeaponCombo/P_Combo_Finish_Untyped_01.P_Combo_Finish_Untyped_01")
      (Components|Activation|Activate _particleskill false))
    (:Defense
      ;[1 1 1] Defense
      (Effects|Components|ParticleSystem|SetTemplate _particleskill "/Game/InfinityBladeEffects/Effects/FX_Ability/Heal/P_Health_Pickup_01.P_Health_Pickup_01")
      (Components|Activation|Activate _particleskill false))
    (:GiveMeTheFireBlast
      (CallFunction|PlayAnimationFireBall))
    (:Exclaimchas
      ;[1 1 1] Exclaimchas
      (Effects|Components|ParticleSystem|SetTemplate _particleskill_4 "/Game/InfinityBladeEffects/Effects/FX_Combat_Base/Enchants/P_Enchant_Cooldowns.P_Enchant_Cooldowns")
      (Components|Activation|Activate _particleskill_4 false))
    (:WhoHeal
      ;[1 1 1] Heal and ShotMana
      (Effects|Components|ParticleSystem|SetTemplate _particleskill_2 "/Game/InfinityBladeEffects/Effects/FX_Ability/Heal/P_Heal_Target.P_Heal_Target")
      (Components|Activation|Activate _particleskill_2 false))
    (:GetHurt
      ;[1 1 1] Get Hurt
      (Effects|Components|ParticleSystem|SetTemplate _particleskill_3 "/Game/InfinityBladeEffects/Effects/FX_Ability/Stun/P_Stun_Stars_Base.P_Stun_Stars_Base")
      (Components|Activation|Activate _particleskill_3 false))))

(fn PutCameraPlayeronView
  (Variables|Default|SetbFindCameraComponentWhenViewTarget true)
  (Game|Player|SetViewTargetwithBlend (Game|GetPlayerController 0) self 1.0 "VTBlend_Linear" 0.0 false))

(fn PlayAnimationFireBall
  (Game|SpawnActorfromClass "/Game/BluePrints/Proyectiles/FireBall.FireBall_C" (Math|Transform|MakeTransform (+ (Transformation|GetActorLocation) "0.000000,0.000000, 0") (Transformation|GetActorRotation)) "Undefined" 0 self))