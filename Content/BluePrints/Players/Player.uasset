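; Player Blueprint that handles the character's appearance and skill effects through callable functions; its own event graph runs no logic.
; ChangeSkin swaps mesh, material and anim class, while ChangeMaterial tints a dynamic material instance.
; ChangeWeapon stores WeaponType and spawns weapon actors onto hand sockets, reusing classes at different scales.
; PlaySkillAnimation maps skill IDs to particle templates or a spawned FireBall, with basic attack effects chosen by WeaponType.
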(event EventBeginPlay)

(event Collision|EventActorBeginOverlap
  (params (OtherActor :type Actor%20Object%20Reference)))

(event EventTick
  (params (DeltaSeconds :type Float%20%28single-precision%29)))

(fn ConstructionScript)

(fn ChangeMaterial
  (params (Color :type Integer))
  (bind _materialdynamicinstance (Variables|Default|GetMaterialDynamicInstance))
  (bind _materialdynamicinstance_2 (Variables|Default|GetMaterialDynamicInstance))
  (switch int Color
    (:Default
      (Rendering|Material|SetVectorParameterValue (Variables|Default|GetMaterialDynamicInstance) "Color" "(R=0.000000,G=0.000000,B=0.000000,A=1.000000)" :!class /Script/Engine.MaterialInstanceDynamic :!label _label))
    (:0
      (Rendering|Material|SetVectorParameterValue _materialdynamicinstance_2 "Color" "(R=1.000000,G=0.000000,B=0.000000,A=1.000000)" :!class /Script/Engine.MaterialInstanceDynamic))
    (:1
      (Rendering|Material|SetVectorParameterValue _materialdynamicinstance_2 "Color" "(R=0.000000,G=1.000000,B=0.000000,A=1.000000)" :!class /Script/Engine.MaterialInstanceDynamic))
    (:2
      (Rendering|Material|SetVectorParameterValue _materialdynamicinstance_2 "Color" "(R=0.000000,G=0.000000,B=1.000000,A=1.000000)" :!class /Script/Engine.MaterialInstanceDynamic))
    (:3
      (Rendering|Material|SetVectorParameterValue _materialdynamicinstance_2 "Color" "(R=1.000000,G=1.000000,B=0.000000,A=1.000000)" :!class /Script/Engine.MaterialInstanceDynamic))
    (:4
      (Rendering|Material|SetVectorParameterValue _materialdynamicinstance "Color" "(R=1.000000,G=0.000000,B=1.000000,A=1.000000)" :!class /Script/Engine.MaterialInstanceDynamic))
    (:5
      (Rendering|Material|SetVectorParameterValue _materialdynamicinstance "Color" "(R=1.000000,G=0.166000,B=0.000000,A=1.000000)" :!class /Script/Engine.MaterialInstanceDynamic))
    (:6
      (Rendering|Material|SetVectorParameterValue _materialdynamicinstance "Color" "(R=0.000000,G=1.000000,B=1.000000,A=1.000000)" :!class /Script/Engine.MaterialInstanceDynamic))
    (:7
      (Rendering|Material|SetVectorParameterValue _materialdynamicinstance "Color" "(R=1.000000,G=1.000000,B=1.000000,A=1.000000)" :!class /Script/Engine.MaterialInstanceDynamic))
    (:8
      (goto _label))))

(fn ChangeSkin
  (params (TypeOfSkin :type Integer))
  (bind _mesh (Variables|Character|GetMesh))
  (switch int TypeOfSkin
    (:0
      (Class|SkinnedMeshComponent|SetSkeletalMesh _mesh "/Game/Models/Geometry/Legionary/Legionary.Legionary" true)
      (Rendering|Material|SetMaterial _mesh 0 "/Game/Models/Geometry/Legionary/MI_Legionario.MI_Legionario")
      (Components|SkeletalMesh|SetAnimInstanceClass (Variables|Character|GetMesh) "/Game/Models/Animations/Legionario_Animation.Legionario_Animation_C"))
    (:1
      (Class|SkinnedMeshComponent|SetSkeletalMesh _mesh "/Game/Models/Geometry/Pistolero/pistolero.pistolero" true)
      (Rendering|Material|SetMaterial _mesh 0 "/Game/Models/Materials/PlayerMaterial_Instance.PlayerMaterial_Instance")
      (Components|SkeletalMesh|SetAnimInstanceClass (Variables|Character|GetMesh) "/Game/Models/Animations/Rango_Animation.Rango_Animation_C"))
    (:2
      (Class|SkinnedMeshComponent|SetSkeletalMesh _mesh "/Game/Models/Geometry/Arquero/arquero_s.arquero_s" true)
      (Rendering|Material|SetMaterial _mesh 0 "/Game/Models/Materials/PlayerMaterial.PlayerMaterial")
      (Components|SkeletalMesh|SetAnimInstanceClass (Variables|Character|GetMesh) "/Game/Models/Animations/Rango_Animation.Rango_Animation_C"))
    (:3
      (Class|SkinnedMeshComponent|SetSkeletalMesh _mesh "/Game/Models/Geometry/Mago/mago.mago" true)
      (Rendering|Material|SetMaterial _mesh 0 "/Game/Models/Materials/PlayerMaterial.PlayerMaterial")
      (Components|SkeletalMesh|SetAnimInstanceClass (Variables|Character|GetMesh) "/Game/Models/Animations/Mago_Animation.Mago_Animation_C"))))

(fn ChangeWeapon
  (params (ID_TypeWeapon :type Integer))
  (bind _returnvalue (Math|Conversions|ToByte(Integer) ID_TypeWeapon))
  (bind _returnvalue_2 (Math|Transform|MakeTransform "0, 0, 0" "0, 0, 0" "1.000000,1.000000,1.000000"))
  (bind _returnvalue_3 (Math|Transform|MakeTransform "0, 0, 0" "0, 0, 0" "0.500000,0.500000,0.500000"))
  (bind _mesh (Variables|Character|GetMesh))
  (bind _mesh_2 (Variables|Character|GetMesh))
  (bind _returnvalue_4 (Utilities|Enum|ByteToEnumTypeWeapons _returnvalue))
  (Variables|Default|SetWeaponType _returnvalue_4)
  (switch Utilities|FlowControl|Switch|SwitchonTypeWeapons _returnvalue_4
    (:SwordAndShield
      ;[1 0 0] Escudo y Espada
      (bind _returnvalue_5 (Game|SpawnActorfromClass "/Game/BluePrints/Weapons/SwordWeapon.SwordWeapon_C" (Math|Transform|MakeTransform "0, 0, 0") "Undefined" 0 0))
      (Transformation|AttachComponentToComponent (Variables|/Game/BluePrints/Weapons/SwordWeapon.SwordWeapon_C|GetWeapon _returnvalue_5) (Variables|Character|GetMesh) "RightHand" "KeepRelative" "KeepRelative" "KeepRelative" true)
      (bind _returnvalue_6 (Game|SpawnActorfromClass "/Game/BluePrints/Weapons/ShieldWeapon_Melee.ShieldWeapon_Melee_C" (Math|Transform|MakeTransform "0, 0, 0") "Undefined" 0 0))
      (Transformation|AttachComponentToComponent (Variables|/Game/BluePrints/Weapons/ShieldWeapon_Melee.ShieldWeapon_Melee_C|GetWeapon _returnvalue_6) (Variables|Character|GetMesh) "LeftHand" "KeepRelative" "KeepRelative" "KeepRelative" true)
      (Variables|Default|SetWeaponRight _returnvalue_5))
    (:Daggers
      ;[1 0 0] Dagas
      (bind _returnvalue_7 (Game|SpawnActorfromClass "/Game/BluePrints/Weapons/SwordWeapon.SwordWeapon_C" _returnvalue_3 "Undefined" 0 0))
      (bind _returnvalue_8 (Game|SpawnActorfromClass "/Game/BluePrints/Weapons/SwordWeapon.SwordWeapon_C" _returnvalue_3 "Undefined" 0 0))
      (Transformation|AttachComponentToComponent (Variables|/Game/BluePrints/Weapons/SwordWeapon.SwordWeapon_C|GetWeapon _returnvalue_7) _mesh "RightHand" "KeepRelative" "KeepRelative" "KeepWorld" true)
      (Transformation|AttachComponentToComponent (Variables|/Game/BluePrints/Weapons/SwordWeapon.SwordWeapon_C|GetWeapon _returnvalue_8) _mesh "LeftHand" "KeepRelative" "KeepRelative" "KeepWorld" true)
      (Variables|Default|SetWeaponRight _returnvalue_7)
      (Variables|Default|SetWeaponLeft _returnvalue_8))
    (:TwoHandSword
      ;[1 0 0] ESPADON
      (bind _returnvalue_9 (Game|SpawnActorfromClass "/Game/BluePrints/Weapons/SwordWeapon.SwordWeapon_C" (Math|Transform|MakeTransform "0, 0, 0" "0, 0, 0" "2.000000,2.000000,1") "Undefined" 0 0))
      (Transformation|AttachComponentToComponent (Variables|/Game/BluePrints/Weapons/SwordWeapon.SwordWeapon_C|GetWeapon _returnvalue_9) (Variables|Character|GetMesh) "RightHand" "KeepRelative" "KeepRelative" "KeepWorld" true)
      (Variables|Default|SetWeaponRight _returnvalue_9))
    (:CrossbowAndShield
      ;[0 0 1] Ballesta y Escudo
      (bind _returnvalue_10 (Game|SpawnActorfromClass "/Game/BluePrints/Weapons/GunWeapon.GunWeapon_C" (Math|Transform|MakeTransform "0, 0, 0") "Undefined" 0 0))
      (Transformation|AttachComponentToComponent (Variables|/Game/BluePrints/Weapons/GunWeapon.GunWeapon_C|GetWeapon _returnvalue_10) (Variables|Character|GetMesh) "RightHand" "KeepRelative" "KeepRelative" "KeepRelative" true)
      (bind _returnvalue_11 (Game|SpawnActorfromClass "/Game/BluePrints/Weapons/ShieldWeapon_Melee.ShieldWeapon_Melee_C" (Math|Transform|MakeTransform "0, 0, 0") "Undefined" 0 0))
      (Transformation|AttachComponentToComponent (Variables|/Game/BluePrints/Weapons/ShieldWeapon_Melee.ShieldWeapon_Melee_C|GetWeapon _returnvalue_11) (Variables|Character|GetMesh) "LeftHand" "KeepRelative" "KeepRelative" "KeepRelative" true)
      (Variables|Default|SetWeaponRight _returnvalue_10))
    (:TwoGuns
      ;[0 0 1] 2 Pistolas
      (bind _returnvalue_12 (Game|SpawnActorfromClass "/Game/BluePrints/Weapons/GunWeapon.GunWeapon_C" _returnvalue_2 "Undefined" 0 0))
      (bind _returnvalue_13 (Game|SpawnActorfromClass "/Game/BluePrints/Weapons/gunWeaponLeft.gunWeaponLeft_C" _returnvalue_2 "Undefined" 0 0))
      (Transformation|AttachComponentToComponent (Variables|/Game/BluePrints/Weapons/GunWeapon.GunWeapon_C|GetWeapon _returnvalue_12) _mesh_2 "RightHand" "KeepRelative" "KeepRelative" "KeepRelative" true)
      (Transformation|AttachComponentToComponent (Variables|/Game/BluePrints/Weapons/gunWeaponLeft.gunWeaponLeft_C|GetWeapon _returnvalue_13) _mesh_2 "LeftHand" "KeepRelative" "KeepRelative" "KeepRelative" true)
      (Variables|Default|SetWeaponRight _returnvalue_13)
      (Variables|Default|SetWeaponLeft _returnvalue_12))
    (:Bow
      ;[0 0 1] ARCO
      (bind _returnvalue_14 (Game|SpawnActorfromClass "/Game/BluePrints/Weapons/BowWeapon_Player.BowWeapon_Player_C" (Math|Transform|MakeTransform "0, 0, 0" "0, 0, 0" "1.000000,1.000000,1") "Undefined" 0 0))
      (Transformation|AttachComponentToComponent (Variables|/Game/BluePrints/Weapons/BowWeapon_Player.BowWeapon_Player_C|GetWeapon _returnvalue_14) (Variables|Character|GetMesh) "LeftHand" "KeepRelative" "KeepRelative" "KeepRelative" true)
      (Variables|Default|SetWeaponRight _returnvalue_14))
    (:WandAndShield
      ;[0 1 0] Varita y Escudo
      (bind _returnvalue_15 (Game|SpawnActorfromClass "/Game/BluePrints/Weapons/StaffWeapon.StaffWeapon_C" (Math|Transform|MakeTransform "0, 0, 0" "0, 0, 0" "1.000000,1.000000,0.500000") "Undefined" 0 0))
      (Transformation|AttachComponentToComponent (Variables|/Game/BluePrints/Weapons/StaffWeapon.StaffWeapon_C|GetWeapon _returnvalue_15) (Variables|Character|GetMesh) "RightHand" "KeepRelative" "KeepRelative" "KeepWorld" true)
      (bind _returnvalue_16 (Game|SpawnActorfromClass "/Game/BluePrints/Weapons/ShieldWeapon.ShieldWeapon_C" (Math|Transform|MakeTransform "0, 0, 0") "Undefined" 0 0))
      (Transformation|AttachComponentToComponent (Variables|/Game/BluePrints/Weapons/ShieldWeapon.ShieldWeapon_C|GetWeapon _returnvalue_16) (Variables|Character|GetMesh) "LeftHand" "KeepRelative" "KeepRelative" "KeepRelative" true)
      (Variables|Default|SetWeaponRight _returnvalue_15))
    (:ScepterAndArcaneBook
      ;[0 1 0] Cetro y Tomo Arcano
      (bind _returnvalue_17 (Game|SpawnActorfromClass "/Game/BluePrints/Weapons/StaffWeapon.StaffWeapon_C" (Math|Transform|MakeTransform "0, 0, 0" "0, 0, 0" "1.000000,1.000000,1") "Undefined" 0 0))
      (Transformation|AttachComponentToComponent (Variables|/Game/BluePrints/Weapons/StaffWeapon.StaffWeapon_C|GetWeapon _returnvalue_17) (Variables|Character|GetMesh) "RightHand" "KeepRelative" "KeepRelative" "KeepRelative" true)
      (Variables|Default|SetWeaponRight _returnvalue_17))
    (:Staff
      ;[0 1 0] Baston
      (bind _returnvalue_18 (Game|SpawnActorfromClass "/Game/BluePrints/Weapons/StaffWeapon.StaffWeapon_C" (Math|Transform|MakeTransform "0, 0, 0" "0, 0, 0" "2.000000,2.000000,1.500000") "Undefined" 0 0))
      (Transformation|AttachComponentToComponent (Variables|/Game/BluePrints/Weapons/StaffWeapon.StaffWeapon_C|GetWeapon _returnvalue_18) (Variables|Character|GetMesh) "RightHand" "KeepRelative" "KeepRelative" "KeepWorld" true)
      (Variables|Default|SetWeaponRight _returnvalue_18))))

(fn PlaySkillAnimation
  (params (ID_Skill :type Integer))
  (bind _particleskill (Variables|Default|GetParticleSKill))
  (bind _particleskill_2 (Variables|Default|GetParticleSKill))
  (switch Utilities|FlowControl|Switch|SwitchonActiveSkills (Utilities|Enum|ByteToEnumActiveSkills (Math|Conversions|ToByte(Integer) ID_Skill))
    (:BasicAttack
      (CallFunction|PlayAnimationBasicAttack))
    (:Defense
      ;[1 1 1] Defense
      (Effects|Components|ParticleSystem|SetTemplate _particleskill_2 "/Game/InfinityBladeEffects/Effects/FX_Ability/Heal/P_Health_Pickup_01.P_Health_Pickup_01")
      (Components|Activation|Activate _particleskill_2 false))
    (:GiveMeTheFireBlast
      (CallFunction|PlayAnimationFireBall))
    (:Exclaimchas
      ;[1 1 1] Exclaim Chas
      (Effects|Components|ParticleSystem|SetTemplate _particleskill_2 "/Game/InfinityBladeEffects/Effects/FX_Combat_Lightning/P_LineToPoint_Proj_Lightning_00.P_LineToPoint_Proj_Lightning_00")
      (Components|Activation|Activate _particleskill_2 false))
    (:BeInCrossroads
      ;[1 1 1] BeInCrossroads
      (Effects|Components|ParticleSystem|SetTemplate _particleskill_2 "/Game/InfinityBladeEffects/Effects/FX_Combat_Ice/P_Player_Frozen_Exit_01.P_Player_Frozen_Exit_01")
      (Components|Activation|Activate _particleskill_2 false))
    (:WhoHeal
      ;[1 1 1] Heal and ShotMana
      (Effects|Components|ParticleSystem|SetTemplate _particleskill_2 "/Game/InfinityBladeEffects/Effects/FX_Ability/Heal/P_Heal_Target.P_Heal_Target" :!label _label)
      (Components|Activation|Activate _particleskill_2 false))
    (:ShotMana
      (goto _label))
    (:GetHurt
      ;[1 1 1] Get Hurt
      (Effects|Components|ParticleSystem|SetTemplate _particleskill "/Game/InfinityBladeEffects/Effects/FX_Ability/Stun/P_Stun_Stars_Base.P_Stun_Stars_Base")
      (Components|Activation|Activate _particleskill false))))

(fn PlayAnimationBasicAttack
  (bind _particleskill (Variables|Default|GetParticleSKill))
  (bind _particleskill_2 (Variables|Default|GetParticleSKill))
  (bind _particleskill_3 (Variables|Default|GetParticleSKill))
  (switch Utilities|FlowControl|Switch|SwitchonTypeWeapons (Variables|Default|GetWeaponType)
    (:SwordAndShield
      ;[1 0 0] Melee
      (Effects|Components|ParticleSystem|SetTemplate _particleskill_2 "/Game/InfinityBladeEffects/Effects/FX_Combat_Base/WeaponCombo/P_Combo_Finish_Untyped_01.P_Combo_Finish_Untyped_01")
      (Components|Activation|Activate _particleskill_2 false))
    (:Daggers
      (Effects|Components|ParticleSystem|SetTemplate _particleskill_2 "/Game/InfinityBladeEffects/Effects/FX_Combat_Base/WeaponCombo/P_Combo_Finish_Untyped_01.P_Combo_Finish_Untyped_01")
      (Components|Activation|Activate _particleskill_2 false))
    (:TwoHandSword
      (Effects|Components|ParticleSystem|SetTemplate _particleskill_2 "/Game/InfinityBladeEffects/Effects/FX_Combat_Base/WeaponCombo/P_Combo_Finish_Untyped_01.P_Combo_Finish_Untyped_01")
      (Components|Activation|Activate _particleskill_2 false))
    (:CrossbowAndShield
      ;[0 0.03478 1] RANGO
      (Effects|Components|ParticleSystem|SetTemplate _particleskill_3 "/Game/InfinityBladeEffects/Effects/FX_Combat_Base/Impact/P_Impact_Enemy_Fire_Strong.P_Impact_Enemy_Fire_Strong")
      (Components|Activation|Activate _particleskill_3 false))
    (:TwoGuns
      (Effects|Components|ParticleSystem|SetTemplate _particleskill_3 "/Game/InfinityBladeEffects/Effects/FX_Combat_Base/Impact/P_Impact_Enemy_Fire_Strong.P_Impact_Enemy_Fire_Strong")
      (Components|Activation|Activate _particleskill_3 false))
    (:Bow
      (Effects|Components|ParticleSystem|SetTemplate _particleskill_3 "/Game/InfinityBladeEffects/Effects/FX_Combat_Base/WeaponCombo/P_Combo_Finish_Untyped_01.P_Combo_Finish_Untyped_01")
      (Components|Activation|Activate _particleskill_3 false))
    (:WandAndShield
      ;[0.08855 1 0] MAGIA
      (Effects|Components|ParticleSystem|SetTemplate _particleskill "/Game/InfinityBladeEffects/Effects/FX_Combat_Base/Enchants/P_Enchant_Cooldowns.P_Enchant_Cooldowns")
      (Components|Activation|Activate _particleskill false))
    (:ScepterAndArcaneBook
      (Effects|Components|ParticleSystem|SetTemplate _particleskill "/Game/InfinityBladeEffects/Effects/FX_Combat_Base/Enchants/P_Enchant_Cooldowns.P_Enchant_Cooldowns")
      (Components|Activation|Activate _particleskill false))
    (:Staff
      (Effects|Components|ParticleSystem|SetTemplate _particleskill "/Game/InfinityBladeEffects/Effects/FX_Combat_Base/Enchants/P_Enchant_Cooldowns.P_Enchant_Cooldowns")
      (Components|Activation|Activate _particleskill false))))

(fn PlayAnimationFireBall
  (Game|SpawnActorfromClass "/Game/BluePrints/Proyectiles/FireBall.FireBall_C" (Math|Transform|MakeTransform (+ (Transformation|GetActorLocation) "0.000000,0.000000, 0") (Transformation|GetActorRotation)) "Undefined" 0 self))