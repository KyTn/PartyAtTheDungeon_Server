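; Server gameplay camera that registers with PD_ServerGameInstance on BeginPlay and can blend in as the first player's view.
; Two zoom functions project player or target positions to screen space and widen the clamped FOV while any fall outside the viewport.
; HideWalls traces from the camera to each player and hides wall actors the game instance returns for the hit location.
; Event-graph calls to zoom and wall hiding are disconnected.
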(event EventBeginPlay
  (bind _aspd_server_game_instance (Utilities|Casting|CastToPD_ServerGameInstance (Game|GetGameInstance)))
  (Class|PDServerGameInstance|CameraRegister _aspd_server_game_instance self))

(event Collision|EventActorBeginOverlap
  (params (OtherActor :type Actor%20Object%20Reference)))

(event EventTick
  (params (DeltaSeconds :type Float%20%28single-precision%29)))

(fn ConstructionScript)

(fn ManageZoomOnlyPlayers
  (params (PositionsToCheck :type Array%20of%20Vectors))
  (while (!= (Utilities|Array|Length PositionsToCheck) (Variables|Default|GetAllInViewport))
    (for _array_element PositionsToCheck
      (bind _returnvalue (Class|ServerCamera|IsinCurrentViewPort (.ScreenLocation (Class|PlayerController|ProjectWorldLocationtoScreen (Game|GetPlayerController 0) _array_element false))))
      (if _returnvalue
        (bind _result (Math|Integer|IncrementInt (Variables|Default|GetAllInViewport))
          (:%20%20
            (Variables|Default|SetAllInViewport _result)))
        (else
          (Camera|SetFieldOfView (Variables|Default|GetCameraComponent) (Math|Float|Clamp(Float) (+ (Variables|Default|GetFOV) 1e+01) 6e+01 1.2e+02)))))))

(fn ManageZoomwithTargetPositions
  (bind _aspd_server_game_instance (Utilities|Casting|CastToPD_ServerGameInstance (Game|GetGameInstance)))
  (bind _returnvalue (Class|PDServerGameInstance|GetTargetPositions _aspd_server_game_instance))
  (while (!= (Utilities|Array|Length _returnvalue) (Variables|Default|GetAllInViewport))
    (for _array_element _returnvalue
      (bind _returnvalue_2 (Class|ServerCamera|IsinCurrentViewPort (.ScreenLocation (Class|PlayerController|ProjectWorldLocationtoScreen (Game|GetPlayerController 0) _array_element false))))
      (if _returnvalue_2
        (bind _result (Math|Integer|IncrementInt (Variables|Default|GetAllInViewport))
          (:%20%20
            (Variables|Default|SetAllInViewport _result)))
        (else
          (Camera|SetFieldOfView (Variables|Default|GetCameraComponent) (Math|Float|Clamp(Float) (+ (Variables|Default|GetFOV) 1e+01) 6e+01 1.2e+02)))))))

(fn HideWalls
  (bind _aspd_server_game_instance (Utilities|Casting|CastToPD_ServerGameInstance (Game|GetGameInstance)))
  (bind _returnvalue (Class|PDServerGameInstance|GetPlayersPositions _aspd_server_game_instance))
  (for _array_element _returnvalue
    (bind _outhit (Collision|LineTraceByChannel (Transformation|GetActorLocation) _array_element "TraceTypeQuery2" false 0 "None"))
    (bind _aspd_server_game_instance_2 (Utilities|Casting|CastToPD_ServerGameInstance (Game|GetGameInstance)))
    (bind _returnvalue_2 (Class|PDServerGameInstance|HiddenActorsBlockPlayers _aspd_server_game_instance_2 (Transformation|GetActorLocation (.HitActor (Collision|BreakHitResult _outhit)))))
    (for _array_element_2 _returnvalue_2
      (bind _asbp_me_wall_actor (Utilities|Casting|CastToBP_ME_WallActor _array_element_2))
      (Rendering|SetActorHiddenInGame _asbp_me_wall_actor true))))

(fn PutCameraPlayeronView
  (Variables|Default|SetbFindCameraComponentWhenViewTarget true)
  (Game|Player|SetViewTargetwithBlend (Game|GetPlayerController 0) self 2.0 "VTBlend_Linear" 0.0 false))