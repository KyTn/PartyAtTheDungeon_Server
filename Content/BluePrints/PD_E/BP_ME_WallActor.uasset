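; Map wall tile actor with a normal block form and thin NS and WE forms, switched by visibility functions.
; Per-side MapSkin values choose fog-capable wall and tile materials for five themes, with Garden variants picked at random.
; Fog functions set FogFinal, and Tick writes a Lerp toward it into every mesh's "Fog" parameter.
; The Lerp takes FogFinal as A, so a small DeltaSeconds × FogVelocity nearly snaps to target.
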(event EventBeginPlay)

(event Collision|EventActorBeginOverlap
  (params (OtherActor :type Actor%20Object%20Reference)))

(event EventTick
  (params (DeltaSeconds :type Float%20%28single-precision%29))
  (Utilities|FlowControl|Sequence
    (:then_0
      (Rendering|Material|SetScalarParameterValueonMaterials (Variables|Default|GetMesh_top) "Fog" (Math|Float|Lerp (Variables|Default|GetFog_Final) (Variables|Default|GetFog_Actual) (* DeltaSeconds (Variables|Default|GetFog_Velocity))))
      (Rendering|Material|SetScalarParameterValueonMaterials (Variables|Default|GetMesh_NE) "Fog" (Math|Float|Lerp (Variables|Default|GetFog_Final) (Variables|Default|GetFog_Actual) (* DeltaSeconds (Variables|Default|GetFog_Velocity))))
      (Rendering|Material|SetScalarParameterValueonMaterials (Variables|Default|GetMesh_SE) "Fog" (Math|Float|Lerp (Variables|Default|GetFog_Final) (Variables|Default|GetFog_Actual) (* DeltaSeconds (Variables|Default|GetFog_Velocity))))
      (Rendering|Material|SetScalarParameterValueonMaterials (Variables|Default|GetMesh_SW) "Fog" (Math|Float|Lerp (Variables|Default|GetFog_Final) (Variables|Default|GetFog_Actual) (* DeltaSeconds (Variables|Default|GetFog_Velocity))))
      (Rendering|Material|SetScalarParameterValueonMaterials (Variables|Default|GetMesh_NW) "Fog" (Math|Float|Lerp (Variables|Default|GetFog_Final) (Variables|Default|GetFog_Actual) (* DeltaSeconds (Variables|Default|GetFog_Velocity)))))
    (:then_1
      (Rendering|Material|SetScalarParameterValueonMaterials (Variables|Default|GetThin_Mesh_E) "Fog" (Math|Float|Lerp (Variables|Default|GetFog_Final) (Variables|Default|GetFog_Actual) (* DeltaSeconds (Variables|Default|GetFog_Velocity))))
      (Rendering|Material|SetScalarParameterValueonMaterials (Variables|Default|GetThin_Mesh_W) "Fog" (Math|Float|Lerp (Variables|Default|GetFog_Final) (Variables|Default|GetFog_Actual) (* DeltaSeconds (Variables|Default|GetFog_Velocity))))
      (Rendering|Material|SetScalarParameterValueonMaterials (Variables|Default|GetThin_Top_WS) "Fog" (Math|Float|Lerp (Variables|Default|GetFog_Final) (Variables|Default|GetFog_Actual) (* DeltaSeconds (Variables|Default|GetFog_Velocity))))
      (Rendering|Material|SetScalarParameterValueonMaterials (Variables|Default|GetThin_Tile_WE_W) "Fog" (Math|Float|Lerp (Variables|Default|GetFog_Final) (Variables|Default|GetFog_Actual) (* DeltaSeconds (Variables|Default|GetFog_Velocity))))
      (Rendering|Material|SetScalarParameterValueonMaterials (Variables|Default|GetThin_Tile_WE_E) "Fog" (Math|Float|Lerp (Variables|Default|GetFog_Final) (Variables|Default|GetFog_Actual) (* DeltaSeconds (Variables|Default|GetFog_Velocity)))))
    (:then_2
      (Rendering|Material|SetScalarParameterValueonMaterials (Variables|Default|GetThin_Mesh_N) "Fog" (Math|Float|Lerp (Variables|Default|GetFog_Final) (Variables|Default|GetFog_Actual) (* DeltaSeconds (Variables|Default|GetFog_Velocity))))
      (Rendering|Material|SetScalarParameterValueonMaterials (Variables|Default|GetThin_Mesh_S) "Fog" (Math|Float|Lerp (Variables|Default|GetFog_Final) (Variables|Default|GetFog_Actual) (* DeltaSeconds (Variables|Default|GetFog_Velocity))))
      (Rendering|Material|SetScalarParameterValueonMaterials (Variables|Default|GetThin_Top_NS) "Fog" (Math|Float|Lerp (Variables|Default|GetFog_Final) (Variables|Default|GetFog_Actual) (* DeltaSeconds (Variables|Default|GetFog_Velocity))))
      (Rendering|Material|SetScalarParameterValueonMaterials (Variables|Default|GetThin_Tile_NS_S) "Fog" (Math|Float|Lerp (Variables|Default|GetFog_Final) (Variables|Default|GetFog_Actual) (* DeltaSeconds (Variables|Default|GetFog_Velocity))))
      (Rendering|Material|SetScalarParameterValueonMaterials (Variables|Default|GetThin_Tile_NS_N) "Fog" (Math|Float|Lerp (Variables|Default|GetFog_Final) (Variables|Default|GetFog_Actual) (* DeltaSeconds (Variables|Default|GetFog_Velocity)))))
    (:then_3
      (Variables|Default|SetFog_Actual (Math|Float|Lerp (Variables|Default|GetFog_Final) (Variables|Default|GetFog_Actual) (* DeltaSeconds (Variables|Default|GetFog_Velocity)))))))

(fn ConstructionScript)

(fn BPChangeMaterialPropertiesMapSkin
  (CallFunction|NormalUpdateMaterials)
  (CallFunction|ThinUpdateMaterials))

(fn BPNormalUpdateMaterials
  (bind _mesh_ne (Variables|Default|GetMesh_NE))
  (bind _mesh_sw (Variables|Default|GetMesh_SW))
  (bind _mesh_se (Variables|Default|GetMesh_SE))
  (bind _mesh_nw (Variables|Default|GetMesh_NW))
  (Utilities|FlowControl|Sequence
    (:then_0
      (switch Utilities|FlowControl|Switch|SwitchonMapSkinType (Variables|Default|GetmapSkin_N)
        (:DUNGEON_NORMAL
          (Rendering|Material|SetMaterial _mesh_ne 0 "/Game/Models/PD_E/ESC/SK_DUNG/WALLS/M_Dungeon_Wall_Fog_Inst.M_Dungeon_Wall_Fog_Inst"))
        (:GARDEN
          (switch int (Math|Random|RandomIntegerinRange 0 2)
            (:0
              (Rendering|Material|SetMaterial _mesh_ne 0 "/Game/Models/PD_E/ESC/SK_GARD/WALLS/1/M_Garden_Wall_01_Fog_Inst.M_Garden_Wall_01_Fog_Inst"))
            (:1
              (Rendering|Material|SetMaterial _mesh_ne 0 "/Game/Models/PD_E/ESC/SK_GARD/WALLS/2/M_Garden_Wall_02_Fog_Inst.M_Garden_Wall_02_Fog_Inst"))
            (:2
              (Rendering|Material|SetMaterial _mesh_ne 0 "/Game/Models/PD_E/ESC/SK_GARD/WALLS/3/M_Garden_Wall_03_Fog_Inst.M_Garden_Wall_03_Fog_Inst"))))
        (:LIBRARY
          (Rendering|Material|SetMaterial _mesh_ne 0 "/Game/Models/PD_E/ESC/SK_LIBR/WALLS/M_Library_Wall_01_Fog_Inst.M_Library_Wall_01_Fog_Inst"))
        (:SACRIFICE
          (Rendering|Material|SetMaterial _mesh_ne 0 "/Game/Models/PD_E/ESC/SK_SACR/WALLS/M_Sacrifice_Wall_01_Fog_Inst.M_Sacrifice_Wall_01_Fog_Inst"))
        (:BOSS
          (Rendering|Material|SetMaterial _mesh_ne 0 "/Game/Models/PD_E/ESC/SK_BOSS/WALLS/M_Boss_Wall_Fog_Inst.M_Boss_Wall_Fog_Inst"))))
    (:then_1
      (switch Utilities|FlowControl|Switch|SwitchonMapSkinType (Variables|Default|GetmapSkin_S)
        (:DUNGEON_NORMAL
          (Rendering|Material|SetMaterial _mesh_sw 0 "/Game/Models/PD_E/ESC/SK_DUNG/WALLS/M_Dungeon_Wall_Fog_Inst.M_Dungeon_Wall_Fog_Inst"))
        (:GARDEN
          (switch int (Math|Random|RandomIntegerinRange 0 2)
            (:0
              (Rendering|Material|SetMaterial _mesh_sw 0 "/Game/Models/PD_E/ESC/SK_GARD/WALLS/1/M_Garden_Wall_01_Fog_Inst.M_Garden_Wall_01_Fog_Inst"))
            (:1
              (Rendering|Material|SetMaterial _mesh_sw 0 "/Game/Models/PD_E/ESC/SK_GARD/WALLS/2/M_Garden_Wall_02_Fog_Inst.M_Garden_Wall_02_Fog_Inst"))
            (:2
              (Rendering|Material|SetMaterial _mesh_sw 0 "/Game/Models/PD_E/ESC/SK_GARD/WALLS/3/M_Garden_Wall_03_Fog_Inst.M_Garden_Wall_03_Fog_Inst"))))
        (:LIBRARY
          (Rendering|Material|SetMaterial _mesh_sw 0 "/Game/Models/PD_E/ESC/SK_LIBR/WALLS/M_Library_Wall_01_Fog_Inst.M_Library_Wall_01_Fog_Inst"))
        (:SACRIFICE
          (Rendering|Material|SetMaterial _mesh_sw 0 "/Game/Models/PD_E/ESC/SK_SACR/WALLS/M_Sacrifice_Wall_01_Fog_Inst.M_Sacrifice_Wall_01_Fog_Inst"))
        (:BOSS
          (Rendering|Material|SetMaterial _mesh_sw 0 "/Game/Models/PD_E/ESC/SK_BOSS/WALLS/M_Boss_Wall_Fog_Inst.M_Boss_Wall_Fog_Inst"))))
    (:then_2
      (switch Utilities|FlowControl|Switch|SwitchonMapSkinType (Variables|Default|GetmapSkin_W)
        (:DUNGEON_NORMAL
          (Rendering|Material|SetMaterial _mesh_se 0 "/Game/Models/PD_E/ESC/SK_DUNG/WALLS/M_Dungeon_Wall_Fog_Inst.M_Dungeon_Wall_Fog_Inst"))
        (:GARDEN
          (switch int (Math|Random|RandomIntegerinRange 0 2)
            (:0
              (Rendering|Material|SetMaterial _mesh_se 0 "/Game/Models/PD_E/ESC/SK_GARD/WALLS/1/M_Garden_Wall_01_Fog_Inst.M_Garden_Wall_01_Fog_Inst"))
            (:1
              (Rendering|Material|SetMaterial _mesh_se 0 "/Game/Models/PD_E/ESC/SK_GARD/WALLS/2/M_Garden_Wall_02_Fog_Inst.M_Garden_Wall_02_Fog_Inst"))
            (:2
              (Rendering|Material|SetMaterial _mesh_se 0 "/Game/Models/PD_E/ESC/SK_GARD/WALLS/3/M_Garden_Wall_03_Fog_Inst.M_Garden_Wall_03_Fog_Inst"))))
        (:LIBRARY
          (Rendering|Material|SetMaterial _mesh_se 0 "/Game/Models/PD_E/ESC/SK_LIBR/WALLS/M_Library_Wall_01_Fog_Inst.M_Library_Wall_01_Fog_Inst"))
        (:SACRIFICE
          (Rendering|Material|SetMaterial _mesh_se 0 "/Game/Models/PD_E/ESC/SK_SACR/WALLS/M_Sacrifice_Wall_01_Fog_Inst.M_Sacrifice_Wall_01_Fog_Inst"))
        (:BOSS
          (Rendering|Material|SetMaterial _mesh_se 0 "/Game/Models/PD_E/ESC/SK_BOSS/WALLS/M_Boss_Wall_Fog_Inst.M_Boss_Wall_Fog_Inst"))))
    (:then_3
      (switch Utilities|FlowControl|Switch|SwitchonMapSkinType (Variables|Default|GetmapSkin_E)
        (:DUNGEON_NORMAL
          (Rendering|Material|SetMaterial _mesh_nw 0 "/Game/Models/PD_E/ESC/SK_DUNG/WALLS/M_Dungeon_Wall_Fog_Inst.M_Dungeon_Wall_Fog_Inst"))
        (:GARDEN
          (switch int (Math|Random|RandomIntegerinRange 0 2)
            (:0
              (Rendering|Material|SetMaterial _mesh_nw 0 "/Game/Models/PD_E/ESC/SK_GARD/WALLS/1/M_Garden_Wall_01_Fog_Inst.M_Garden_Wall_01_Fog_Inst"))
            (:1
              (Rendering|Material|SetMaterial _mesh_nw 0 "/Game/Models/PD_E/ESC/SK_GARD/WALLS/2/M_Garden_Wall_02_Fog_Inst.M_Garden_Wall_02_Fog_Inst"))
            (:2
              (Rendering|Material|SetMaterial _mesh_nw 0 "/Game/Models/PD_E/ESC/SK_GARD/WALLS/3/M_Garden_Wall_03_Fog_Inst.M_Garden_Wall_03_Fog_Inst"))))
        (:LIBRARY
          (Rendering|Material|SetMaterial _mesh_nw 0 "/Game/Models/PD_E/ESC/SK_LIBR/WALLS/M_Library_Wall_01_Fog_Inst.M_Library_Wall_01_Fog_Inst"))
        (:SACRIFICE
          (Rendering|Material|SetMaterial _mesh_nw 0 "/Game/Models/PD_E/ESC/SK_SACR/WALLS/M_Sacrifice_Wall_01_Fog_Inst.M_Sacrifice_Wall_01_Fog_Inst"))
        (:BOSS
          (Rendering|Material|SetMaterial _mesh_nw 0 "/Game/Models/PD_E/ESC/SK_BOSS/WALLS/M_Boss_Wall_Fog_Inst.M_Boss_Wall_Fog_Inst"))))))

(fn BPNNotVisible
  (Rendering|SetVisibility (Variables|Default|GetMesh_NE) false false))

(fn BPWNotVisible
  (Rendering|SetVisibility (Variables|Default|GetMesh_SE) false false))

(fn BPSNotVisible
  (Rendering|SetVisibility (Variables|Default|GetMesh_SW) false false))

(fn BPENotVisible
  (Rendering|SetVisibility (Variables|Default|GetMesh_NW) false false))

(fn BPThinNSVisible
  (Rendering|SetVisibility (Variables|Default|GetMesh_NE) false false)
  (Rendering|SetVisibility (Variables|Default|GetMesh_SE) false false)
  (Rendering|SetVisibility (Variables|Default|GetMesh_SW) false false)
  (Rendering|SetVisibility (Variables|Default|GetMesh_NW) false false)
  (Rendering|SetVisibility (Variables|Default|GetMesh_top) false false)
  (Rendering|SetVisibility (Variables|Default|GetThin_Mesh_E) false false)
  (Rendering|SetVisibility (Variables|Default|GetThin_Mesh_W) false false)
  (Rendering|SetVisibility (Variables|Default|GetThin_Top_WS) false false)
  (Rendering|SetVisibility (Variables|Default|GetThin_Tile_WE_W) false false)
  (Rendering|SetVisibility (Variables|Default|GetThin_Tile_WE_E) false false)
  (Rendering|SetVisibility (Variables|Default|GetThin_Mesh_N) true false)
  (Rendering|SetVisibility (Variables|Default|GetThin_Mesh_S) true false)
  (Rendering|SetVisibility (Variables|Default|GetThin_Top_NS) true false)
  (Rendering|SetVisibility (Variables|Default|GetThin_Tile_NS_N) true false)
  (Rendering|SetVisibility (Variables|Default|GetThin_Tile_NS_S) true false))

(fn BPThinWEVisible
  (Rendering|SetVisibility (Variables|Default|GetMesh_NE) false false)
  (Rendering|SetVisibility (Variables|Default|GetMesh_SE) false false)
  (Rendering|SetVisibility (Variables|Default|GetMesh_SW) false false)
  (Rendering|SetVisibility (Variables|Default|GetMesh_NW) false false)
  (Rendering|SetVisibility (Variables|Default|GetMesh_top) false false)
  (Rendering|SetVisibility (Variables|Default|GetThin_Mesh_E) true false)
  (Rendering|SetVisibility (Variables|Default|GetThin_Mesh_W) true false)
  (Rendering|SetVisibility (Variables|Default|GetThin_Top_WS) true false)
  (Rendering|SetVisibility (Variables|Default|GetThin_Tile_WE_W) true false)
  (Rendering|SetVisibility (Variables|Default|GetThin_Tile_WE_E) true false)
  (Rendering|SetVisibility (Variables|Default|GetThin_Mesh_N) false false)
  (Rendering|SetVisibility (Variables|Default|GetThin_Mesh_S) false false)
  (Rendering|SetVisibility (Variables|Default|GetThin_Top_NS) false false)
  (Rendering|SetVisibility (Variables|Default|GetThin_Tile_NS_N) false false)
  (Rendering|SetVisibility (Variables|Default|GetThin_Tile_NS_S) false false))

(fn BPNormalAllVisible
  (Rendering|SetVisibility (Variables|Default|GetMesh_NE) true false)
  (Rendering|SetVisibility (Variables|Default|GetMesh_SE) true false)
  (Rendering|SetVisibility (Variables|Default|GetMesh_SW) true false)
  (Rendering|SetVisibility (Variables|Default|GetMesh_NW) true false)
  (Rendering|SetVisibility (Variables|Default|GetMesh_top) true false)
  (Rendering|SetVisibility (Variables|Default|GetThin_Mesh_E) false false)
  (Rendering|SetVisibility (Variables|Default|GetThin_Mesh_W) false false)
  (Rendering|SetVisibility (Variables|Default|GetThin_Top_WS) false false)
  (Rendering|SetVisibility (Variables|Default|GetThin_Tile_WE_W) false false)
  (Rendering|SetVisibility (Variables|Default|GetThin_Tile_WE_E) false false)
  (Rendering|SetVisibility (Variables|Default|GetThin_Mesh_N) false false)
  (Rendering|SetVisibility (Variables|Default|GetThin_Mesh_S) false false)
  (Rendering|SetVisibility (Variables|Default|GetThin_Top_NS) false false)
  (Rendering|SetVisibility (Variables|Default|GetThin_Tile_NS_N) false false)
  (Rendering|SetVisibility (Variables|Default|GetThin_Tile_NS_S) false false))

(fn BPThinUpdateMaterials
  (bind _thin_tile_ns_n (Variables|Default|GetThin_Tile_NS_N))
  (bind _thin_tile_ns_s (Variables|Default|GetThin_Tile_NS_S))
  (bind _thin_tile_we_w (Variables|Default|GetThin_Tile_WE_W))
  (bind _thin_tile_we_e (Variables|Default|GetThin_Tile_WE_E))
  (bind _thin_mesh_n (Variables|Default|GetThin_Mesh_N))
  (bind _thin_mesh_s (Variables|Default|GetThin_Mesh_S))
  (bind _thin_mesh_w (Variables|Default|GetThin_Mesh_W))
  (bind _thin_mesh_e (Variables|Default|GetThin_Mesh_E))
  (Utilities|FlowControl|Sequence
    (:then_0
      (switch Utilities|FlowControl|Switch|SwitchonMapSkinType (Variables|Default|GetmapSkin_N)
        (:DUNGEON_NORMAL
          (Rendering|Material|SetMaterial _thin_mesh_n 0 "/Game/Models/PD_E/ESC/SK_DUNG/WALLS/M_Dungeon_Wall_Fog_Inst.M_Dungeon_Wall_Fog_Inst")
          (Rendering|Material|SetMaterial _thin_tile_ns_n 0 "/Game/Models/PD_E/ESC/SK_DUNG/TILES/Normal_Tile/M_Dungeon_NormalTile_Fog_Inst.M_Dungeon_NormalTile_Fog_Inst"))
        (:GARDEN
          (Utilities|FlowControl|Sequence
            (:then_0
              (switch int (Math|Random|RandomIntegerinRange 0 2)
                (:0
                  (Rendering|Material|SetMaterial _thin_mesh_n 0 "/Game/Models/PD_E/ESC/SK_GARD/WALLS/1/M_Garden_Wall_01_Fog_Inst.M_Garden_Wall_01_Fog_Inst"))
                (:1
                  (Rendering|Material|SetMaterial _thin_mesh_n 0 "/Game/Models/PD_E/ESC/SK_GARD/WALLS/2/M_Garden_Wall_02_Fog_Inst.M_Garden_Wall_02_Fog_Inst"))
                (:2
                  (Rendering|Material|SetMaterial _thin_mesh_n 0 "/Game/Models/PD_E/ESC/SK_GARD/WALLS/3/M_Garden_Wall_03_Fog_Inst.M_Garden_Wall_03_Fog_Inst"))))
            (:then_1
              (switch int (Math|Random|RandomIntegerinRange 0 2)
                (:0
                  (Rendering|Material|SetMaterial _thin_tile_ns_n 0 "/Game/Models/PD_E/ESC/SK_GARD/TILES/Normal_Tile/1/M_Garden_NormalTile_Fog_Inst.M_Garden_NormalTile_Fog_Inst"))
                (:1
                  (Rendering|Material|SetMaterial _thin_tile_ns_n 0 "/Game/Models/PD_E/ESC/SK_GARD/TILES/Normal_Tile/2-piedras/M_Garden_NormalTile_02_Fog_Inst.M_Garden_NormalTile_02_Fog_Inst"))
                (:2
                  (Rendering|Material|SetMaterial _thin_tile_ns_n 0 "/Game/Models/PD_E/ESC/SK_GARD/TILES/Normal_Tile/2-piedras/M_Garden_NormalTile_02_Fog_Inst.M_Garden_NormalTile_02_Fog_Inst"))))))
        (:LIBRARY
          (Rendering|Material|SetMaterial _thin_mesh_n 0 "/Game/Models/PD_E/ESC/SK_LIBR/WALLS/M_Library_Wall_01_Fog_Inst.M_Library_Wall_01_Fog_Inst")
          (Rendering|Material|SetMaterial _thin_tile_ns_n 0 "/Game/Models/PD_E/ESC/SK_LIBR/TILES/Normal_Tile/M_Library_NormalTile_Fog_Inst.M_Library_NormalTile_Fog_Inst"))
        (:SACRIFICE
          (Rendering|Material|SetMaterial _thin_mesh_n 0 "/Game/Models/PD_E/ESC/SK_SACR/WALLS/M_Sacrifice_Wall_01_Fog_Inst.M_Sacrifice_Wall_01_Fog_Inst")
          (Rendering|Material|SetMaterial _thin_tile_ns_n 0 "/Game/Models/PD_E/ESC/SK_SACR/TILES/Normal_Tile/M_Sacrifice_NormalTile_Fog_Inst.M_Sacrifice_NormalTile_Fog_Inst"))
        (:BOSS
          (Rendering|Material|SetMaterial _thin_mesh_n 0 "/Game/Models/PD_E/ESC/SK_BOSS/WALLS/M_Boss_Wall_Fog_Inst.M_Boss_Wall_Fog_Inst")
          (Rendering|Material|SetMaterial _thin_tile_ns_n 0 "/Game/Models/PD_E/ESC/SK_BOSS/TILES/Normal_Tile/M_Boss_NormalTile_Fog_Inst.M_Boss_NormalTile_Fog_Inst"))))
    (:then_1
      (switch Utilities|FlowControl|Switch|SwitchonMapSkinType (Variables|Default|GetmapSkin_S)
        (:DUNGEON_NORMAL
          (Rendering|Material|SetMaterial _thin_mesh_s 0 "/Game/Models/PD_E/ESC/SK_DUNG/WALLS/M_Dungeon_Wall_Fog_Inst.M_Dungeon_Wall_Fog_Inst")
          (Rendering|Material|SetMaterial _thin_tile_ns_s 0 "/Game/Models/PD_E/ESC/SK_DUNG/TILES/Normal_Tile/M_Dungeon_NormalTile_Fog_Inst.M_Dungeon_NormalTile_Fog_Inst"))
        (:GARDEN
          (Utilities|FlowControl|Sequence
            (:then_0
              (switch int (Math|Random|RandomIntegerinRange 0 2)
                (:0
                  (Rendering|Material|SetMaterial _thin_mesh_s 0 "/Game/Models/PD_E/ESC/SK_GARD/WALLS/1/M_Garden_Wall_01_Fog_Inst.M_Garden_Wall_01_Fog_Inst"))
                (:1
                  (Rendering|Material|SetMaterial _thin_mesh_s 0 "/Game/Models/PD_E/ESC/SK_GARD/WALLS/2/M_Garden_Wall_02_Fog_Inst.M_Garden_Wall_02_Fog_Inst"))
                (:2
                  (Rendering|Material|SetMaterial _thin_mesh_s 0 "/Game/Models/PD_E/ESC/SK_GARD/WALLS/3/M_Garden_Wall_03_Fog_Inst.M_Garden_Wall_03_Fog_Inst"))))
            (:then_1
              (switch int (Math|Random|RandomIntegerinRange 0 2)
                (:0
                  (Rendering|Material|SetMaterial _thin_tile_ns_s 0 "/Game/Models/PD_E/ESC/SK_GARD/TILES/Normal_Tile/1/M_Garden_NormalTile_Fog_Inst.M_Garden_NormalTile_Fog_Inst"))
                (:1
                  (Rendering|Material|SetMaterial _thin_tile_ns_s 0 "/Game/Models/PD_E/ESC/SK_GARD/TILES/Normal_Tile/2-piedras/M_Garden_NormalTile_02_Fog_Inst.M_Garden_NormalTile_02_Fog_Inst"))
                (:2
                  (Rendering|Material|SetMaterial _thin_tile_ns_s 0 "/Game/Models/PD_E/ESC/SK_GARD/TILES/Normal_Tile/2-piedras/M_Garden_NormalTile_02_Fog_Inst.M_Garden_NormalTile_02_Fog_Inst"))))))
        (:LIBRARY
          (Rendering|Material|SetMaterial _thin_mesh_s 0 "/Game/Models/PD_E/ESC/SK_LIBR/WALLS/M_Library_Wall_01_Fog_Inst.M_Library_Wall_01_Fog_Inst")
          (Rendering|Material|SetMaterial _thin_tile_ns_s 0 "/Game/Models/PD_E/ESC/SK_LIBR/TILES/Normal_Tile/M_Library_NormalTile_Fog_Inst.M_Library_NormalTile_Fog_Inst"))
        (:SACRIFICE
          (Rendering|Material|SetMaterial _thin_mesh_s 0 "/Game/Models/PD_E/ESC/SK_SACR/WALLS/M_Sacrifice_Wall_01_Fog_Inst.M_Sacrifice_Wall_01_Fog_Inst")
          (Rendering|Material|SetMaterial _thin_tile_ns_s 0 "/Game/Models/PD_E/ESC/SK_SACR/TILES/Normal_Tile/M_Sacrifice_NormalTile_Fog_Inst.M_Sacrifice_NormalTile_Fog_Inst"))
        (:BOSS
          (Rendering|Material|SetMaterial _thin_mesh_s 0 "/Game/Models/PD_E/ESC/SK_BOSS/WALLS/M_Boss_Wall_Fog_Inst.M_Boss_Wall_Fog_Inst")
          (Rendering|Material|SetMaterial _thin_tile_ns_s 0 "/Game/Models/PD_E/ESC/SK_BOSS/TILES/Normal_Tile/M_Boss_NormalTile_Fog_Inst.M_Boss_NormalTile_Fog_Inst"))))
    (:then_2
      (switch Utilities|FlowControl|Switch|SwitchonMapSkinType (Variables|Default|GetmapSkin_W)
        (:DUNGEON_NORMAL
          (Rendering|Material|SetMaterial _thin_mesh_w 0 "/Game/Models/PD_E/ESC/SK_DUNG/WALLS/M_Dungeon_Wall_Fog_Inst.M_Dungeon_Wall_Fog_Inst")
          (Rendering|Material|SetMaterial _thin_tile_we_w 0 "/Game/Models/PD_E/ESC/SK_DUNG/TILES/Normal_Tile/M_Dungeon_NormalTile_Fog_Inst.M_Dungeon_NormalTile_Fog_Inst"))
        (:GARDEN
          (Utilities|FlowControl|Sequence
            (:then_0
              (switch int (Math|Random|RandomIntegerinRange 0 2)
                (:0
                  (Rendering|Material|SetMaterial _thin_mesh_w 0 "/Game/Models/PD_E/ESC/SK_GARD/WALLS/1/M_Garden_Wall_01_Fog_Inst.M_Garden_Wall_01_Fog_Inst"))
                (:1
                  (Rendering|Material|SetMaterial _thin_mesh_w 0 "/Game/Models/PD_E/ESC/SK_GARD/WALLS/2/M_Garden_Wall_02_Fog_Inst.M_Garden_Wall_02_Fog_Inst"))
                (:2
                  (Rendering|Material|SetMaterial _thin_mesh_w 0 "/Game/Models/PD_E/ESC/SK_GARD/WALLS/3/M_Garden_Wall_03_Fog_Inst.M_Garden_Wall_03_Fog_Inst"))))
            (:then_1
              (switch int (Math|Random|RandomIntegerinRange 0 2)
                (:0
                  (Rendering|Material|SetMaterial _thin_tile_we_w 0 "/Game/Models/PD_E/ESC/SK_GARD/TILES/Normal_Tile/1/M_Garden_NormalTile_Fog_Inst.M_Garden_NormalTile_Fog_Inst"))
                (:1
                  (Rendering|Material|SetMaterial _thin_tile_we_w 0 "/Game/Models/PD_E/ESC/SK_GARD/TILES/Normal_Tile/2-piedras/M_Garden_NormalTile_02_Fog_Inst.M_Garden_NormalTile_02_Fog_Inst"))
                (:2
                  (Rendering|Material|SetMaterial _thin_tile_we_w 0 "/Game/Models/PD_E/ESC/SK_GARD/TILES/Normal_Tile/2-piedras/M_Garden_NormalTile_02_Fog_Inst.M_Garden_NormalTile_02_Fog_Inst"))))))
        (:LIBRARY
          (Rendering|Material|SetMaterial _thin_mesh_w 0 "/Game/Models/PD_E/ESC/SK_LIBR/WALLS/M_Library_Wall_01_Fog_Inst.M_Library_Wall_01_Fog_Inst")
          (Rendering|Material|SetMaterial _thin_tile_we_w 0 "/Game/Models/PD_E/ESC/SK_LIBR/TILES/Normal_Tile/M_Library_NormalTile_Fog_Inst.M_Library_NormalTile_Fog_Inst"))
        (:SACRIFICE
          (Rendering|Material|SetMaterial _thin_mesh_w 0 "/Game/Models/PD_E/ESC/SK_SACR/WALLS/M_Sacrifice_Wall_01_Fog_Inst.M_Sacrifice_Wall_01_Fog_Inst")
          (Rendering|Material|SetMaterial _thin_tile_we_w 0 "/Game/Models/PD_E/ESC/SK_SACR/TILES/Normal_Tile/M_Sacrifice_NormalTile_Fog_Inst.M_Sacrifice_NormalTile_Fog_Inst"))
        (:BOSS
          (Rendering|Material|SetMaterial _thin_mesh_w 0 "/Game/Models/PD_E/ESC/SK_BOSS/WALLS/M_Boss_Wall_Fog_Inst.M_Boss_Wall_Fog_Inst")
          (Rendering|Material|SetMaterial _thin_tile_we_w 0 "/Game/Models/PD_E/ESC/SK_BOSS/TILES/Normal_Tile/M_Boss_NormalTile_Fog_Inst.M_Boss_NormalTile_Fog_Inst"))))
    (:then_3
      (switch Utilities|FlowControl|Switch|SwitchonMapSkinType (Variables|Default|GetmapSkin_E)
        (:DUNGEON_NORMAL
          (Rendering|Material|SetMaterial _thin_mesh_e 0 "/Game/Models/PD_E/ESC/SK_DUNG/WALLS/M_Dungeon_Wall_Fog_Inst.M_Dungeon_Wall_Fog_Inst")
          (Rendering|Material|SetMaterial _thin_tile_we_e 0 "/Game/Models/PD_E/ESC/SK_DUNG/TILES/Normal_Tile/M_Dungeon_NormalTile_Fog_Inst.M_Dungeon_NormalTile_Fog_Inst"))
        (:GARDEN
          (Utilities|FlowControl|Sequence
            (:then_0
              (switch int (Math|Random|RandomIntegerinRange 0 2)
                (:0
                  (Rendering|Material|SetMaterial _thin_mesh_e 0 "/Game/Models/PD_E/ESC/SK_GARD/WALLS/1/M_Garden_Wall_01_Fog_Inst.M_Garden_Wall_01_Fog_Inst"))
                (:1
                  (Rendering|Material|SetMaterial _thin_mesh_e 0 "/Game/Models/PD_E/ESC/SK_GARD/WALLS/2/M_Garden_Wall_02_Fog_Inst.M_Garden_Wall_02_Fog_Inst"))
                (:2
                  (Rendering|Material|SetMaterial _thin_mesh_e 0 "/Game/Models/PD_E/ESC/SK_GARD/WALLS/3/M_Garden_Wall_03_Fog_Inst.M_Garden_Wall_03_Fog_Inst"))))
            (:then_1
              (switch int (Math|Random|RandomIntegerinRange 0 2)
                (:0
                  (Rendering|Material|SetMaterial _thin_tile_we_e 0 "/Game/Models/PD_E/ESC/SK_GARD/TILES/Normal_Tile/1/M_Garden_NormalTile_Fog_Inst.M_Garden_NormalTile_Fog_Inst"))
                (:1
                  (Rendering|Material|SetMaterial _thin_tile_we_e 0 "/Game/Models/PD_E/ESC/SK_GARD/TILES/Normal_Tile/2-piedras/M_Garden_NormalTile_02_Fog_Inst.M_Garden_NormalTile_02_Fog_Inst"))
                (:2
                  (Rendering|Material|SetMaterial _thin_tile_we_e 0 "/Game/Models/PD_E/ESC/SK_GARD/TILES/Normal_Tile/2-piedras/M_Garden_NormalTile_02_Fog_Inst.M_Garden_NormalTile_02_Fog_Inst"))))))
        (:LIBRARY
          (Rendering|Material|SetMaterial _thin_mesh_e 0 "/Game/Models/PD_E/ESC/SK_LIBR/WALLS/M_Library_Wall_01_Fog_Inst.M_Library_Wall_01_Fog_Inst")
          (Rendering|Material|SetMaterial _thin_tile_we_e 0 "/Game/Models/PD_E/ESC/SK_LIBR/TILES/Normal_Tile/M_Library_NormalTile_Fog_Inst.M_Library_NormalTile_Fog_Inst"))
        (:SACRIFICE
          (Rendering|Material|SetMaterial _thin_mesh_e 0 "/Game/Models/PD_E/ESC/SK_SACR/WALLS/M_Sacrifice_Wall_01_Fog_Inst.M_Sacrifice_Wall_01_Fog_Inst")
          (Rendering|Material|SetMaterial _thin_tile_we_e 0 "/Game/Models/PD_E/ESC/SK_SACR/TILES/Normal_Tile/M_Sacrifice_NormalTile_Fog_Inst.M_Sacrifice_NormalTile_Fog_Inst"))
        (:BOSS
          (Rendering|Material|SetMaterial _thin_mesh_e 0 "/Game/Models/PD_E/ESC/SK_BOSS/WALLS/M_Boss_Wall_Fog_Inst.M_Boss_Wall_Fog_Inst")
          (Rendering|Material|SetMaterial _thin_tile_we_e 0 "/Game/Models/PD_E/ESC/SK_BOSS/TILES/Normal_Tile/M_Boss_NormalTile_Fog_Inst.M_Boss_NormalTile_Fog_Inst"))))))

(fn BPACTIVEFOG
  (Variables|Default|SetFog_Final 1.0))

(fn BPDEACTIVEFOG
  (Variables|Default|SetFog_Final 0.0))