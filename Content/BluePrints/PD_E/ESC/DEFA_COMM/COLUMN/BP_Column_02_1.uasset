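; Column map-piece Blueprint with a column mesh and a floor tile mesh that supports fogging and map skins.
; The map-skin function sets the tile's fog material per dungeon theme, choosing randomly among Garden variants.
; Activate and deactivate functions set the fog target to one or zero.
; Tick pushes a Lerp from target toward current value into both meshes' "Fog" parameter, so small alphas land near the target.
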(event EventBeginPlay)

(event Collision|EventActorBeginOverlap
  (params (OtherActor :type Actor%20Object%20Reference)))

(event EventTick
  (params (DeltaSeconds :type Float%20%28single-precision%29))
  (Rendering|Material|SetScalarParameterValueonMaterials (Variables|Default|GetMesh) "Fog" (Math|Float|Lerp (Variables|Default|GetFog_Final) (Variables|Default|GetFog_Actual) (* DeltaSeconds (Variables|Default|GetFog_Velocity))))
  (Rendering|Material|SetScalarParameterValueonMaterials (Variables|Default|GetMesh_Tile) "Fog" (Math|Float|Lerp (Variables|Default|GetFog_Final) (Variables|Default|GetFog_Actual) (* DeltaSeconds (Variables|Default|GetFog_Velocity))))
  (Variables|Default|SetFog_Actual (Math|Float|Lerp (Variables|Default|GetFog_Final) (Variables|Default|GetFog_Actual) (* DeltaSeconds (Variables|Default|GetFog_Velocity)))))

(fn ConstructionScript)

(fn BPChangeMaterialPropertiesMapSkin
  (bind _mesh_tile (Variables|Default|GetMesh_Tile))
  (bind _returnvalue (Class|PDEElementActor|GetMaterialSkin))
  (switch Utilities|FlowControl|Switch|SwitchonMapSkinType _returnvalue
    (:DUNGEON_NORMAL
      (Rendering|Material|SetMaterial _mesh_tile 0 "/Game/Models/PD_E/ESC/SK_DUNG/TILES/Normal_Tile/M_Dungeon_NormalTile_Fog_Inst.M_Dungeon_NormalTile_Fog_Inst"))
    (:GARDEN
      (switch int (Math|Random|RandomIntegerinRange 0 2)
        (:0
          (Rendering|Material|SetMaterial _mesh_tile 0 "/Game/Models/PD_E/ESC/SK_GARD/TILES/Normal_Tile/1/M_Garden_NormalTile_Fog_Inst.M_Garden_NormalTile_Fog_Inst"))
        (:1
          (Rendering|Material|SetMaterial _mesh_tile 0 "/Game/Models/PD_E/ESC/SK_GARD/TILES/Normal_Tile/2-piedras/M_Garden_NormalTile_02_Fog_Inst.M_Garden_NormalTile_02_Fog_Inst"))
        (:2
          (Rendering|Material|SetMaterial _mesh_tile 0 "/Game/Models/PD_E/ESC/SK_GARD/TILES/Normal_Tile/1/M_Garden_NormalTile_Fog_Inst.M_Garden_NormalTile_Fog_Inst"))))
    (:LIBRARY
      (Rendering|Material|SetMaterial _mesh_tile 0 "/Game/Models/PD_E/ESC/SK_LIBR/TILES/Normal_Tile/M_Library_NormalTile_Fog_Inst.M_Library_NormalTile_Fog_Inst"))
    (:SACRIFICE
      (Rendering|Material|SetMaterial _mesh_tile 0 "/Game/Models/PD_E/ESC/SK_SACR/TILES/Normal_Tile/M_Sacrifice_NormalTile_Fog_Inst.M_Sacrifice_NormalTile_Fog_Inst"))
    (:BOSS
      (Rendering|Material|SetMaterial _mesh_tile 0 "/Game/Models/PD_E/ESC/SK_BOSS/TILES/Normal_Tile/M_Boss_NormalTile_Fog_Inst.M_Boss_NormalTile_Fog_Inst"))))

(fn BPACTIVATEFOG
  (Variables|Default|SetFog_Final 1.0))

(fn BPDEACTIVATEFOG
  (Variables|Default|SetFog_Final 0.0))