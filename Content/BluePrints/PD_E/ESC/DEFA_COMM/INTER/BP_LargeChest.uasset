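; BP_LargeChest is a large chest actor with callable functions to open, close and rotate it.
; Opening activates the WhenFua component and deactivates ChestMesh, and closing reverses this through component activation alone, without visibility or animation calls.
; Three rotation functions set the mesh to fixed relative rotations in quarter-turn steps.
; Its event graph and construction script are empty, so the Blueprint never calls these functions itself.
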(event EventBeginPlay)

(event Collision|EventActorBeginOverlap
  (params (OtherActor :type Actor%20Object%20Reference)))

(event EventTick
  (params (DeltaSeconds :type Float%20%28single-precision%29)))

(fn ConstructionScript)

(fn BPOPENCHEST
  (Components|Activation|Activate (Variables|Default|GetWhenFua) false)
  (Components|Activation|Deactivate (Variables|Default|Getchest_mesh)))

(fn BPRotate90
  (Transformation|SetRelativeRotation (Variables|Default|Getchest_mesh) "0,90.000000, 0" false false))

(fn BPRotate180
  (Transformation|SetRelativeRotation (Variables|Default|Getchest_mesh) "0,180.000000, 0" false false))

(fn BPRotate270
  (Transformation|SetRelativeRotation (Variables|Default|Getchest_mesh) "0,270.000000, 0" false false))

(fn BPCLOSECHEST
  (Components|Activation|Activate (Variables|Default|Getchest_mesh) false)
  (Components|Activation|Deactivate (Variables|Default|GetWhenFua)))