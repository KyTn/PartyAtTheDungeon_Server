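; Obstruction tile Blueprint that dresses its floor tile to match the map skin and can show or clear a fog effect.
; The skin function sets a fog-capable tile material, randomly picking a variant for Dungeon, Garden and Sacrifice.
; Activate and deactivate functions set the fog target, which Tick blends into both meshes' "Fog" parameter.
; The Lerp takes the target as A, so small alphas land almost on target rather than easing.
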(event EventBeginPlay)

(event Collision|EventActorBeginOverlap
  (params (OtherActor :type Actor%20Object%20Reference)))

(event EventTick
  (params (DeltaSeconds :type Float%20%28single-precision%29))
  (Rendering|Material|SetScalarParameterValueonMaterials (Variables|Default|GetObject_Mesh) "Fog" (Math|Float|Lerp (Variables|Default|GetFog_Final) (Variables|Default|GetFog_Actual) (* DeltaSeconds (Variables|Default|GetFog_Velocity))))
  (Rendering|Material|SetScalarParameterValueonMaterials (Variables|Default|GetTile_Mesh) "Fog" (Math|Float|Lerp (Variables|Default|GetFog_Final) (Variables|Default|GetFog_Actual) (* DeltaSeconds (Variables|Default|GetFog_Velocity))))
  (Variables|Default|SetFog_Actual (Math|Float|Lerp (Variables|Default|GetFog_Final) (Variables|Default|GetFog_Actual) (* DeltaSeconds (Variables|Default|GetFog_Velocity)))))

(fn ConstructionScript)

(fn BPChangeMaterialPropertiesMapSkin
  (bind _tile_mesh (Variables|Default|GetTile_Mesh))
  (bind _returnvalue (Class|PDEElementActor|GetMaterialSkin))
  (switch Utilities|FlowControl|Switch|SwitchonMapSkinType _returnvalue
    (:DUNGEON_NORMAL
      (switch int (Math|Random|RandomIntegerinRange 0 2)
        (:0
          (Rendering|Material|SetMaterial _tile_mesh 0 "/Game/Models/PD_E/ESC/SK_DUNG/TILES/Normal_Tile/01/M_Dungeon_NormalTile_Fog_Inst_01.M_Dungeon_NormalTile_Fog_Inst_01"))
        (:1
          (Rendering|Material|SetMaterial _tile_mesh 0 "/Game/Models/PD_E/ESC/SK_DUNG/TILES/Normal_Tile/02/M_Dungeon_NormalTile_Fog_Inst_02.M_Dungeon_NormalTile_Fog_Inst_02"))
        (:2
          (Rendering|Material|SetMaterial _tile_mesh 0 "/Game/Models/PD_E/ESC/SK_DUNG/TILES/Normal_Tile/03/M_Dungeon_NormalTile_Fog_Inst_03.M_Dungeon_NormalTile_Fog_Inst_03"))))
    (:GARDEN
      (switch int (Math|Random|RandomIntegerinRange 0 2)
        (:0
          (Rendering|Material|SetMaterial _tile_mesh 0 "/Game/Models/PD_E/ESC/SK_GARD/TILES/Normal_Tile/1/M_Garden_NormalTile_Fog_Inst.M_Garden_NormalTile_Fog_Inst"))
        (:1
          (Rendering|Material|SetMaterial _tile_mesh 0 "/Game/Models/PD_E/ESC/SK_GARD/TILES/Normal_Tile/2-piedras/M_Garden_NormalTile_02_Fog_Inst.M_Garden_NormalTile_02_Fog_Inst"))
        (:2
          (Rendering|Material|SetMaterial _tile_mesh 0 "/Game/Models/PD_E/ESC/SK_GARD/TILES/Normal_Tile/1/M_Garden_NormalTile_Fog_Inst.M_Garden_NormalTile_Fog_Inst"))))
    (:LIBRARY
      (Rendering|Material|SetMaterial _tile_mesh 0 "/Game/Models/PD_E/ESC/SK_LIBR/TILES/Normal_Tile/M_Library_NormalTile_Fog_Inst.M_Library_NormalTile_Fog_Inst"))
    (:SACRIFICE
      (switch int (Math|Random|RandomIntegerinRange 0 2)
        (:0
          (Rendering|Material|SetMaterial _tile_mesh 0 "/Game/Models/PD_E/ESC/SK_SACR/TILES/Normal_Tile/01/M_Sacrifice_NormalTile_Fog_Inst_01.M_Sacrifice_NormalTile_Fog_Inst_01"))
        (:1
          (Rendering|Material|SetMaterial _tile_mesh 0 "/Game/Models/PD_E/ESC/SK_SACR/TILES/Normal_Tile/02/M_Sacrifice_NormalTile_Fog_Inst_02.M_Sacrifice_NormalTile_Fog_Inst_02"))
        (:2
          (Rendering|Material|SetMaterial _tile_mesh 0 "/Game/Models/PD_E/ESC/SK_SACR/TILES/Normal_Tile/03/M_Sacrifice_NormalTile_Fog_Inst_03.M_Sacrifice_NormalTile_Fog_Inst_03"))))
    (:BOSS
      (Rendering|Material|SetMaterial _tile_mesh 0 "/Game/Models/PD_E/ESC/SK_BOSS/TILES/Normal_Tile/M_Boss_NormalTile_Fog_Inst.M_Boss_NormalTile_Fog_Inst"))))

(fn BPACTIVATEFOG
  (Variables|Default|SetFog_Final 1.0))

(fn BPDEACTIVATEFOG
  (Variables|Default|SetFog_Final 0.0))