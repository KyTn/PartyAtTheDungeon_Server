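; Fence wall prop for what appears to be a boss level, exposing helper functions to adjust its placement and visibility.
; Functions hide ObjectMesh or set the Pivot to fixed quarter-turn relative rotations.
; A thin-wall function shifts the mesh along its local offset on X, guarded by IsToThinWall so it applies only once.
; The event graph and construction script are empty, so nothing here calls these functions.
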(event EventBeginPlay)

(event Collision|EventActorBeginOverlap
  (params (OtherActor :type Actor%20Object%20Reference)))

(event EventTick
  (params (DeltaSeconds :type Float%20%28single-precision%29)))

(fn ConstructionScript)

(fn BPNotVisible
  (Rendering|SetVisibility (Variables|Default|GetObject_Mesh) false false))

(fn BPRotate90
  (Transformation|SetRelativeRotation (Variables|Default|GetPivot) "0,90.000000, 0" false false))

(fn BPRotate180
  (Transformation|SetRelativeRotation (Variables|Default|GetPivot) "0,180.000000, 0" false false))

(fn BPRotate270
  (Transformation|SetRelativeRotation (Variables|Default|GetPivot) "0,270.000000, 0" false false))

(fn BPMoveProptoThinWall
  (if (not (Variables|Default|GetisToThinWall))
    (Transformation|AddRelativeLocation (Variables|Default|GetObject_Mesh) "-40.000000, 0, 0" false false)
    (Variables|Default|SetisToThinWall true)))