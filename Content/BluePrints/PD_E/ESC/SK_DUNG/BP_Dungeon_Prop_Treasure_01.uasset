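; Treasure dungeon prop Blueprint that drives a "Fog" material parameter on its object and tile meshes.
; Activate and deactivate functions switch the fog target between on and off.
; Tick lerps from that target toward the current value by delta time times velocity, so small alphas land near the target.
; The result is written to both meshes' materials and stored as the current fog.
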(event EventBeginPlay)

(event Collision|EventActorBeginOverlap
  (params (OtherActor :type Actor%20Object%20Reference)))

(event EventTick
  (params (DeltaSeconds :type Float%20%28single-precision%29))
  (Rendering|Material|SetScalarParameterValueonMaterials (Variables|Default|GetObject_Mesh) "Fog" (Math|Float|Lerp (Variables|Default|GetFog_Final) (Variables|Default|GetFog_Actual) (* DeltaSeconds (Variables|Default|GetFog_Velocity))))
  (Rendering|Material|SetScalarParameterValueonMaterials (Variables|Default|GetTile_Mesh) "Fog" (Math|Float|Lerp (Variables|Default|GetFog_Final) (Variables|Default|GetFog_Actual) (* DeltaSeconds (Variables|Default|GetFog_Velocity))))
  (Variables|Default|SetFog_Actual (Math|Float|Lerp (Variables|Default|GetFog_Final) (Variables|Default|GetFog_Actual) (* DeltaSeconds (Variables|Default|GetFog_Velocity)))))

(fn ConstructionScript)

(fn BPACTIVATEFOG
  (Variables|Default|SetFog_Final 1.0))

(fn BPDEACTIVATEFOG
  (Variables|Default|SetFog_Final 0.0))