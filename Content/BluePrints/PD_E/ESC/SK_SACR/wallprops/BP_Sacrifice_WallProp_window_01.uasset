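; Window wall prop Blueprint with a tile mesh and an object mesh, with functions to hide the object or rotate its pivot in quarter turns.
; A one-time offset moves the object mesh to fit a thin wall.
; Fog activate and deactivate functions set a target value.
; Tick lerps from that target toward the current value by delta time times velocity, driving both meshes' "Fog" material parameter.
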(event EventBeginPlay)

(event Collision|EventActorBeginOverlap
  (params (OtherActor :type Actor%20Object%20Reference)))

(event EventTick
  (params (DeltaSeconds :type Float%20%28single-precision%29))
  (Rendering|Material|SetScalarParameterValueonMaterials (Variables|Default|GetTile_Mesh) "Fog" (Math|Float|Lerp (Variables|Default|GetFog_Final) (Variables|Default|GetFog_Actual) (* DeltaSeconds (Variables|Default|GetFog_Velocity))))
  (Rendering|Material|SetScalarParameterValueonMaterials (Variables|Default|GetObject_Mesh) "Fog" (Math|Float|Lerp (Variables|Default|GetFog_Final) (Variables|Default|GetFog_Actual) (* DeltaSeconds (Variables|Default|GetFog_Velocity))))
  (Variables|Default|SetFog_Actual (Math|Float|Lerp (Variables|Default|GetFog_Final) (Variables|Default|GetFog_Actual) (* DeltaSeconds (Variables|Default|GetFog_Velocity)))))

(fn ConstructionScript)

(fn BPNotVisible
  (Rendering|SetVisibility (Variables|Default|GetObject_Mesh) false false))

(fn BPRotate90
  (Transformation|SetRelativeRotation (Variables|Default|GetPivot) "0,90.000000, 0" false false))

(fn BPRotate180
  (Transformation|SetRelativeRotation (Variables|Default|GetPivot) "0,180.000000, 0" false false))

(fn BPRotate270
  (Transformation|SetRelativeRotation (Variables|Default|GetPivot) "0,270.000000, 0" false false))

(fn BPMoveProptoThinWall
  (if (not (Variables|Default|GetisToThinWall))
    (Transformation|AddRelativeLocation (Variables|Default|GetObject_Mesh) "-40.000000, 0, 0" false false)
    (Variables|Default|SetisToThinWall true)))

(fn BPACTIVATEFOG
  (Variables|Default|SetFog_Final 1.0))

(fn BPDEACTIVATEFOG
  (Variables|Default|SetFog_Final 0.0))